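; Player shooter character that moves, carries one tagged item on a hand socket and can drop it to the ground.
; Pickup flags guns or healing salve by comparing against the first actor of each class.
; Left click restores health or fires a camera line trace damaging MyEnemyToFire_BP, with a looping timer for rifle auto-fire.
; Tick pauses into a death screen at zero health; Tab toggles the item spawn menu, V self-damages.
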(event `InputAction|Jump`
  (params (Key :type "Key Structure"))
  ;[1 1 1] BaseInput
  (:`Pressed`
    (`self.Jump`))
  (:`Released`
    (`self.StopJumping`)))

(event `InputAxis|Turn`
  (params (AxisValue :type "Float (single-precision)"))
  ;[1 1 1] BaseInput
  (`self.AddControllerYawInput` (/ AxisValue 2.0)))

(event `InputAction|PickUp`
  (params (Key :type "Key Structure"))
  (bind _holding_item (`self.Holding Item`))
  ;[1 1 1] PickUp
  (:`Pressed`
    (if (not (`self.is holding smth`))
      (for _array_element (`self.GetOverlappingActors` "/Script/Engine.Actor")
        (if (`self.ActorHasTag` _array_element "Pickupable")
          (bind _output_get (set `self.Holding Item` _array_element))
          (`self.K2_AttachToComponent` _output_get (`self.Mesh`) "WeaponHere" "SnapToTarget" "SnapToTarget" "KeepWorld" true)
          (set `self.is holding smth` true)
          (bind _outactors (`GameplayStatics.GetAllActorsOfClass` "/Game/PickItems/Pistol/Pistol_BP.Pistol_BP_C"))
          (bind _outactors_2 (`GameplayStatics.GetAllActorsOfClass` "/Game/PickItems/HealingSalve/HealingSalve_BP.HealingSalve_BP_C"))
          (bind _outactors_3 (`GameplayStatics.GetAllActorsOfClass` "/Game/PickItems/Rifle/Rifle_BP.Rifle_BP_C"))
          (if (or (== _holding_item (`|GetArrayItem` _outactors)) (== _holding_item (`|GetArrayItem` _outactors_3)))
            (set `self.is gun` true)
            (break)
            (elif (== _holding_item (`|GetArrayItem` _outactors_2))
              (set `self.is usable` true)
              (break)
              (else
                (break)))))))))

(event `InputAxis|LookUp`
  (params (AxisValue :type "Float (single-precision)"))
  ;[1 1 1] BaseInput
  (`self.AddControllerPitchInput` (/ AxisValue 2.0)))

(event `InputAxis|MoveForward`
  (params (AxisValue :type "Float (single-precision)"))
  ;[1 1 1] BaseInput
  (`self.AddMovementInput` (`KismetMathLibrary.GetForwardVector` (`KismetMathLibrary.MakeRotator` 0.0 0.0 (.yaw (`self.GetControlRotation`)))) AxisValue))

(event `InputAction|Drop`
  (params (Key :type "Key Structure"))
  (:`Pressed`
    (`self.DropItem`)))

(event `InputAxis|MoveRight`
  (params (AxisValue :type "Float (single-precision)"))
  ;[1 1 1] BaseInput
  (`self.AddMovementInput` (`KismetMathLibrary.GetRightVector` (`KismetMathLibrary.MakeRotator` 0.0 0.0 (.yaw (`self.GetControlRotation`)))) AxisValue))

(event `Key|LeftMouseButton`
  (params (Key :type "Key Structure"))
  (bind _returnvalue (`GameplayStatics.GetPlayerCameraManager` 0))
  (bind _returnvalue_2 (`PlayerCameraManager.GetCameraLocation` _returnvalue))
  (:`Pressed`
    (if (`self.is holding smth`)
      (if (`self.is usable`)
        (`KismetSystemLibrary.PrintString` "usable")
        (bind _output_get (set `self.Current Health` 100.0))
        (`KismetSystemLibrary.PrintString` (`KismetStringLibrary.Conv_DoubleToString` _output_get))
        (elif (`self.is gun`)
          (`KismetSystemLibrary.PrintString` "gun")
          (bind _outactors (`GameplayStatics.GetAllActorsOfClass` "/Game/PickItems/Rifle/Rifle_BP.Rifle_BP_C"))
          (if (== (`|GetArrayItem` _outactors) (`self.Holding Item`))
            (set `self.DependsOnGun` 0.1)
            (bind _returnvalue_3 (`KismetSystemLibrary.K2_SetTimerDelegate` (delegate `Firing`) (`self.DependsOnGun`) true)))
          (`GameplayStatics.SpawnSound2D` "/Game/SFX/RifleSound.RifleSound" 1.0 1.0 0.0 null :!label _label)
          (bind _outhit (`KismetSystemLibrary.LineTraceSingle` :`Start` _returnvalue_2 :`End` (+ _returnvalue_2 (* (`KismetMathLibrary.GetForwardVector` (`PlayerCameraManager.GetCameraRotation` _returnvalue)) 10000.0)) :`TraceChannel` "TraceTypeQuery1" :`DrawDebugType` "ForDuration"))
          (bind _asmy_enemy_to_fire_bp (cast `/Game/Targets/MyEnemyToFire_BP` (`.HitActor` (`GameplayStatics.BreakHitResult` _outhit))))
          (set `/Game/Targets/MyEnemyToFire_BP.Health` (- (`/Game/Targets/MyEnemyToFire_BP.Health` _asmy_enemy_to_fire_bp) 25.0) _asmy_enemy_to_fire_bp)
          (else
            (`KismetSystemLibrary.PrintString` "other"))))))
  (:`Released`
    (`KismetSystemLibrary.K2_ClearAndInvalidateTimerHandle` _returnvalue_3)))

(event `self.ReceiveTick`
  (params (DeltaSeconds :type "Float (single-precision)"))
  (if (<= (`self.Current Health`) 0.0)
    (`GameplayStatics.SetGamePaused` true)
    (bind _returnvalue (`|CreateWidget` "/Game/UI/DeathScreen_UI.DeathScreen_UI_C"))
    (`UserWidget.AddToViewport` _returnvalue 0)
    (set `PlayerController.bShowMouseCursor` true (`GameplayStatics.GetPlayerController` 0))))

(event `Firing`
  (goto _label))

(event `Key|V`
  (params (Key :type "Key Structure"))
  (:`Pressed`
    (set `self.Current Health` (- (`self.Current Health`) 1.0))))

(event `Key|Tab`
  (params (Key :type "Key Structure"))
  (bind _returnvalue (`GameplayStatics.GetPlayerController` 0))
  (:`Pressed`
    (`/Engine/EditorBlueprintResources/StandardMacros.FlipFlop`
      (:`A`
        (bind _returnvalue_2 (`|CreateWidget` "/Game/UI/SpawnItems_UI.SpawnItems_UI_C"))
        (`UserWidget.AddToViewport` _returnvalue_2 0)
        (set `PlayerController.bShowMouseCursor` true _returnvalue))
      (:`B`
        (bind _foundwidgets (`WidgetBlueprintLibrary.GetAllWidgetsOfClass` "/Game/UI/SpawnItems_UI.SpawnItems_UI_C"))
        (`Widget.RemoveFromParent` (`|GetArrayItem` _foundwidgets))
        (set `PlayerController.bShowMouseCursor` false _returnvalue)))))

(fn `DropItem`
  (bind _holding_item (`self.Holding Item`))
  ;[1 1 1] DropItem
  (if (`self.is holding smth`)
    (bind (_outhit _returnvalue) (`KismetSystemLibrary.LineTraceSingle` (`self.K2_GetActorLocation`) (- (`self.K2_GetActorLocation`) (0.0 0.0 500.0)) "TraceTypeQuery1"))
    (if _returnvalue
      (`self.K2_DetachFromActor` _holding_item "KeepWorld" "KeepWorld" "KeepWorld")
      (`self.K2_SetActorTransform` _holding_item (`KismetMathLibrary.MakeTransform` (`.Location` (`GameplayStatics.BreakHitResult` _outhit))) false false)
      (set `self.is holding smth` false)
      (set `self.is usable` false)
      (set `self.is gun` false))))

(fn `UserConstructionScript`)