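; Homing fireball projectile that chases the player character and damages it on contact.
; Each Tick it moves toward the player's current location at Speed, without sweeping.
; Overlapping a MainShooter_BP with its Sphere directly subtracts a fixed amount from CurrentHealth and destroys the fireball.
; Otherwise it destroys itself after a short delay from BeginPlay.
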(event `self.ReceiveTick`
  (params (DeltaSeconds :type "Float (single-precision)"))
  (bind _returnvalue (`self.K2_GetActorLocation` (`GameplayStatics.GetPlayerCharacter` 0)))
  (`self.K2_AddActorWorldOffset` (* (`KismetMathLibrary.Normal` (- _returnvalue (`self.K2_GetActorLocation` self))) (* DeltaSeconds (`self.speed`))))
  (set `self.Last Position` _returnvalue))

(event `self.ReceiveBeginPlay`
  (`KismetSystemLibrary.Delay` 2.0)
  (`self.K2_DestroyActor`))

(event `self.Sphere.OnComponentBeginOverlap`
  (params (OverlappedComponent :type "PrimitiveComponent Object Reference") (OtherActor :type "Actor Object Reference") (OtherComp :type "PrimitiveComponent Object Reference") (OtherBodyIndex :type Integer) (bFromSweep :type Boolean) (SweepResult :type "HitResult Structure (by ref)"))
  (bind _asmain_shooter_bp (cast `/Game/MainCharacter/MainShooter_BP` OtherActor))
  (set `/Game/MainCharacter/MainShooter_BP.Current Health` (- (`/Game/MainCharacter/MainShooter_BP.Current Health` _asmain_shooter_bp) 25.0) _asmain_shooter_bp)
  (`self.K2_DestroyActor`))

(event `self.Sphere1.OnComponentHit`
  (params (HitComponent :type "PrimitiveComponent Object Reference") (OtherActor :type "Actor Object Reference") (OtherComp :type "PrimitiveComponent Object Reference") (NormalImpulse :type "Vector Structure") (Hit :type "HitResult Structure (by ref)")))

(event `self.Sphere1.OnComponentEndOverlap`
  (params (OverlappedComponent :type "PrimitiveComponent Object Reference") (OtherActor :type "Actor Object Reference") (OtherComp :type "PrimitiveComponent Object Reference") (OtherBodyIndex :type Integer)))

(fn `UserConstructionScript`)